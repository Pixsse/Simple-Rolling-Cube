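; BP_RollingCube is a player-controlled cube that moves through Enhanced Input.
; On BeginPlay it adds the IMC_Player mapping context to its player controller's local subsystem.
; Four directional input actions each pass a direction to RollingCubeComponent.UpdateCubeMovement, which handles the movement, so the Blueprint itself only routes input.
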(event Input|EnhancedActionEvents|EnhancedInputActionIA_MoveBackward
  (params (ActionValue :type Boolean) (ElapsedSeconds :type Float%20%28double-precision%29) (TriggeredSeconds :type Float%20%28double-precision%29) (InputAction :type Input%20Action%20Object%20Reference :default "/Game/Miscs/Inputs/IA_MoveBackward.IA_MoveBackward"))
  ;[0.4093 0.4062 1 0] Movement Inputs
  (Class|RollingCubeComponent|UpdateCubeMovement (Variables|Default|GetRollingCubeComponent) "Backward"))

(event Input|EnhancedActionEvents|EnhancedInputActionIA_MoveForward
  (params (ActionValue :type Boolean) (ElapsedSeconds :type Float%20%28double-precision%29) (TriggeredSeconds :type Float%20%28double-precision%29) (InputAction :type Input%20Action%20Object%20Reference :default "/Game/Miscs/Inputs/IA_MoveForward.IA_MoveForward"))
  ;[0.4093 0.4062 1 0] Movement Inputs
  (Class|RollingCubeComponent|UpdateCubeMovement (Variables|Default|GetRollingCubeComponent) "Forward"))

(event Input|EnhancedActionEvents|EnhancedInputActionIA_MoveLeft
  (params (ActionValue :type Boolean) (ElapsedSeconds :type Float%20%28double-precision%29) (TriggeredSeconds :type Float%20%28double-precision%29) (InputAction :type Input%20Action%20Object%20Reference :default "/Game/Miscs/Inputs/IA_MoveLeft.IA_MoveLeft"))
  ;[0.4093 0.4062 1 0] Movement Inputs
  (Class|RollingCubeComponent|UpdateCubeMovement (Variables|Default|GetRollingCubeComponent) "Left"))

(event Input|EnhancedActionEvents|EnhancedInputActionIA_MoveRight
  (params (ActionValue :type Boolean) (ElapsedSeconds :type Float%20%28double-precision%29) (TriggeredSeconds :type Float%20%28double-precision%29) (InputAction :type Input%20Action%20Object%20Reference :default "/Game/Miscs/Inputs/IA_MoveRight.IA_MoveRight"))
  ;[0.4093 0.4062 1 0] Movement Inputs
  (Class|RollingCubeComponent|UpdateCubeMovement (Variables|Default|GetRollingCubeComponent) "Right"))

(event EventBeginPlay
  ;[0.4093 0.4062 1 0] Add Mapping Context
  (bind _asplayer_controller (Utilities|Casting|CastToPlayerController (Pawn|GetController)))
  (Input|AddMappingContext (PlayerController|LocalPlayerSubsystems|GetEnhancedInputLocalPlayerSubsystem _asplayer_controller) "/Game/Miscs/Inputs/IMC_Player.IMC_Player" 0 "(bIgnoreAllPressedKeysUntilRelease=True,bForceImmediately=False,bNotifyUserSettings=False)"))

(fn ConstructionScript)